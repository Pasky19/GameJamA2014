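; Player controller for a zombie runner, handling arrow-key prompts, brain eating, obstacle spawning and gamepad power-ups.
; Arrow presses are checked against ZombieHud's expected key to set its failure flag.
; MoveToCerveau spawns a brain in a random lane and moves the character to it for button-mash eating.
; Tick runs slowdown, speed-boost and destruction timers; obstacle helpers pick random types, though ObstacleGrandLong is unreachable through a duplicated index check.
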(event Custom|MoveToCerveau
  (bind _cerveau (Variables|Default|GetCerveau))
  (bind _returnvalue (Transformation|GetActorLocation _cerveau))
  (bind (_x _y) (Math|Vector|BreakVector _returnvalue))
  ;[1 1 1] Spawn un cerveau
  (CallFunction|SpawnCerveau)
  (Variables|/Game/Blueprints/MyCharacter.MyCharacter_C|SetIsEating (Variables|Default|GetMyCharacter) true)
  (Components|MoveComponentTo (VehicleSound|GetRootComponent (Variables|Default|GetMyCharacter)) (Math|Vector|MakeVector (- _x 5e+01) _y (.Z (Math|Vector|BreakVector (Transformation|GetActorLocation)))) "0, 0, 0" false false 1.0))

(event Custom|SlowCharacter
  ;[1 1 1] Slow character custom event
  (Variables|/Script/Engine.CharacterMovementComponent|SetMaxWalkSpeed (Variables|/Script/Engine.Character|GetCharacterMovement (Variables|Default|GetMyCharacter)) (- (Variables|Default|GetTempMaxSpeed) 3e+02))
  (Variables|Default|SetTempMaxSpeed (- (Variables|Default|GetTempMaxSpeed) 3e+02)))

(event EventTick
  (params (DeltaSeconds :type Float%20%28single-precision%29))
  (bind _mycharacter (Variables|Default|GetMyCharacter))
  (CallFunction|RalentirCharacter DeltaSeconds)
  (CallFunction|DecelererCharacter DeltaSeconds)
  (CallFunction|DestructionObstacles DeltaSeconds)
  (if (Variables|Default|GetDeceleration)
    (Components|MoveComponentTo (Variables|/Game/Blueprints/MyCharacter.MyCharacter_C|GetCameraBoom _mycharacter) (* (Transformation|GetActorForwardVector _mycharacter) 25.0) "0, 0, 0" false false 0.5)
    (Variables|Default|SetDeceleration false)))

(event EventBeginPlay
  (bind _aszombiehud_c (Utilities|Casting|CastToZombieHud (HUD|GetHUD)))
  (Variables|Default|SetHUD _aszombiehud_c)
  (Variables|Default|SetTimer (Variables|/Game/Blueprints/ZombieHud.ZombieHud_C|GetDelayNextkey (Variables|Default|GetHUD)))
  (bind _asmycharacter_c (Utilities|Casting|CastToMyCharacter (Pawn|GetControlledPawn)))
  (Variables|Default|SetMyCharacter _asmycharacter_c)
  (Variables|Default|SetYDepartCharacter (.Y (Math|Vector|BreakVector (Transformation|GetActorLocation (Variables|Default|GetMyCharacter)))))
  (Variables|Default|SetTempMaxSpeed (Variables|/Script/Engine.CharacterMovementComponent|GetMaxWalkSpeed (Variables|/Script/Engine.Character|GetCharacterMovement (Variables|Default|GetMyCharacter)))))

(event Input|KeyboardEvents|Up
  (:Pressed
    (CallFunction|OnTimer?RightName? "Up")
    (Default|InitializeFleche (Variables|Default|GetHUD))))

(event Input|KeyboardEvents|Down
  (:Pressed
    (CallFunction|OnTimer?RightName? "Down")
    (Default|InitializeFleche (Variables|Default|GetHUD))))

(event Input|KeyboardEvents|Left
  (:Pressed
    (CallFunction|OnTimer?RightName? "Left")
    (Default|InitializeFleche (Variables|Default|GetHUD))))

(event Input|KeyboardEvents|Right
  (:Pressed
    (CallFunction|OnTimer?RightName? "Right")
    (Default|InitializeFleche (Variables|Default|GetHUD))))

(event Input|GamepadEvents|GamepadFaceButtonTop
  (bind _mycharacter (Variables|Default|GetMyCharacter))
  (:Pressed
    (CallFunction|AccelererCharacter)
    (Components|MoveComponentTo (Variables|/Game/Blueprints/MyCharacter.MyCharacter_C|GetCameraBoom _mycharacter) (* (Transformation|GetActorForwardVector _mycharacter) -2e+02) "0, 0, 0" false false 0.5)))

(event Input|GamepadEvents|GamepadFaceButtonLeft
  ;[1 1 1] Appuyer sur x dix fois pour continuer
  (:Pressed
    (if (Variables|/Game/Blueprints/MyCharacter.MyCharacter_C|GetIsEating (Variables|Default|GetMyCharacter))
      (if (<= (Variables|Default|GetButtonPressCount) 10)
        (Variables|Default|SetButtonPressCount (+ (Variables|Default|GetButtonPressCount) 1))
        (else
          (Variables|/Game/Blueprints/MyCharacter.MyCharacter_C|SetIsEating (Variables|Default|GetMyCharacter) false)
          (Actor|DestroyActor (Variables|Default|GetCerveau))
          (Variables|Default|SetButtonPressCount 0))))))

(event Input|GamepadEvents|GamepadFaceButtonLeft
  (:Pressed
    (if (not (Variables|/Game/Blueprints/MyCharacter.MyCharacter_C|GetIsEating (Variables|Default|GetMyCharacter)))
      (CallFunction|InterrompreCombo))))

(event Input|GamepadEvents|GamepadFaceButtonRight
  (:Pressed
    (if (Variables|Default|GetDestructionDisponible)
      (Variables|Default|SetDestructionActive true)
      (Variables|Default|SetDestructionDisponible false)
      (Variables|/Game/Blueprints/ZombieHud.ZombieHud_C|SetDejaAfficherVitesse (Variables|Default|GetHUD) false))))

(fn ConstructionScript)

(fn OnTimer?RightName?
  (params (TouchName :type Name))
  (bind _hud (Variables|Default|GetHUD))
  (bind _hud_2 (Variables|Default|GetHUD))
  (if (Variables|/Game/Blueprints/ZombieHud.ZombieHud_C|GetGo? _hud)
    (if (Utilities|Name|Equal(Name) TouchName (Variables|/Game/Blueprints/ZombieHud.ZombieHud_C|GetKeyName _hud))
      (Variables|/Game/Blueprints/ZombieHud.ZombieHud_C|SetFailed _hud_2 false)
      (else
        (Variables|/Game/Blueprints/ZombieHud.ZombieHud_C|SetFailed _hud_2 true)))))

(fn ChooseRandomObstacle
  (Variables|Default|SetRandomObstacle (Math|Random|RandomInteger 4))
  (if (== (Variables|Default|GetRandomObstacle) 0)
    (Variables|Default|SetObstacle "/Game/Blueprints/Game/ObstaclePetitCourt.ObstaclePetitCourt_C")
    (elif (== (Variables|Default|GetRandomObstacle) 1)
      (Variables|Default|SetObstacle "/Game/Blueprints/Game/ObstaclePetitLong.ObstaclePetitLong_C")
      (elif (== (Variables|Default|GetRandomObstacle) 2)
        (Variables|Default|SetObstacle "/Game/Blueprints/Game/ObstacleGrandCourt.ObstacleGrandCourt_C")
        (elif (== (Variables|Default|GetRandomObstacle) 2)
          (Variables|Default|SetObstacle "/Game/Blueprints/Game/ObstacleGrandLong.ObstacleGrandLong_C"))))))

(fn SpawnObstacleCourt
  (bind _returnvalue (Pawn|GetControlledPawn))
  (bind _returnvalue_2 (Transformation|GetActorLocation _returnvalue))
  (bind (_x _y) (Math|Vector|BreakVector _returnvalue_2))
  (Variables|Default|SetSpawnPositionObstacle (Math|Vector|MakeVector (+ _x 5e+02) _y 123.15))
  (Game|SpawnActorfromClass (Variables|Default|GetObstacle) (Math|Conversions|ToTransform(Vector) (Variables|Default|GetSpawnPositionObstacle)) false))

(fn SpawnObstacleLong
  (bind _returnvalue (Pawn|GetControlledPawn))
  (bind _returnvalue_2 (Pawn|GetControlledPawn))
  (bind _returnvalue_3 (Transformation|GetActorLocation _returnvalue))
  (bind _returnvalue_4 (Transformation|GetActorLocation _returnvalue_2))
  (bind (_x _y) (Math|Vector|BreakVector _returnvalue_3))
  (bind (_x_2 _y_2) (Math|Vector|BreakVector _returnvalue_4))
  (bind _returnvalue_5 (- _y_2 2.5e+02))
  (bind _returnvalue_6 (+ _y 2.5e+02))
  (Variables|Default|SetRandomLeftRight (Math|Random|RandomInteger 2))
  (if (== (Variables|Default|GetRandomLeftRight) 0)
    (Variables|Default|SetPosObstacle _returnvalue_5)
    (Variables|Default|SetSpawnPositionObstacle (Math|Vector|MakeVector (+ _x_2 5e+02) _returnvalue_5 123.15))
    (else
      (Variables|Default|SetPosObstacle _returnvalue_6)
      (Variables|Default|SetSpawnPositionObstacle (Math|Vector|MakeVector (+ _x 5e+02) _returnvalue_6 123.15))))
  (Game|SpawnActorfromClass (Variables|Default|GetObstacle) (Math|Conversions|ToTransform(Vector) (Variables|Default|GetSpawnPositionObstacle)) false))

(fn SpawnCerveau
  (CallFunction|PositionCerveau)
  (Variables|Default|SetSpawnPositionObstacle (Math|Vector|MakeVector (+ (.X (Math|Vector|BreakVector (Transformation|GetActorLocation (Variables|Default|GetMyCharacter)))) 5e+02) (+ (Variables|Default|GetYDepartCharacter) (Variables|Default|GetPositionY)) 123.15))
  (bind _returnvalue (Game|SpawnActorfromClass "/Game/Blueprints/Game/Cerveau.Cerveau_C" (Math|Conversions|ToTransform(Vector) (Variables|Default|GetSpawnPositionObstacle)) false))
  (Variables|Default|SetCerveau _returnvalue))

(fn PositionCerveau
  (bind _mycharacter (Variables|Default|GetMyCharacter))
  (bind _mycharacter_2 (Variables|Default|GetMyCharacter))
  (Variables|Default|SetRandomCerveau (Math|Random|RandomInteger 3))
  (if (== (Variables|Default|GetRandomCerveau) 0)
    (Variables|Default|SetPositionY -5e+02)
    (Variables|/Game/Blueprints/MyCharacter.MyCharacter_C|SetRightCount _mycharacter_2 -1)
    (Variables|/Game/Blueprints/MyCharacter.MyCharacter_C|SetLeftCount _mycharacter 1)
    (elif (== (Variables|Default|GetRandomCerveau) 1)
      (Variables|Default|SetPositionY 0.0)
      (Variables|/Game/Blueprints/MyCharacter.MyCharacter_C|SetRightCount _mycharacter_2 0)
      (Variables|/Game/Blueprints/MyCharacter.MyCharacter_C|SetLeftCount _mycharacter 0)
      (elif (== (Variables|Default|GetRandomCerveau) 2)
        (Variables|Default|SetPositionY 5e+02)
        (Variables|/Game/Blueprints/MyCharacter.MyCharacter_C|SetRightCount _mycharacter_2 1)
        (Variables|/Game/Blueprints/MyCharacter.MyCharacter_C|SetLeftCount _mycharacter -1)))))

(fn SpawnObstacle
  ;[1 1 1] Spawn Obstacle au random
  (CallFunction|ChooseRandomObstacle)
  (if (Utilities|ClassIsChildOf (Variables|Default|GetObstacle) "/Game/Blueprints/Game/ObstaclePetitCourt.ObstaclePetitCourt_C")
    (CallFunction|SpawnObstacleCourt)
    (elif (Utilities|ClassIsChildOf (Variables|Default|GetObstacle) "/Game/Blueprints/Game/ObstacleGrandCourt.ObstacleGrandCourt_C")
      (CallFunction|SpawnObstacleCourt)
      (elif (Utilities|ClassIsChildOf (Variables|Default|GetObstacle) "/Game/Blueprints/Game/ObstaclePetitLong.ObstaclePetitLong_C")
        (CallFunction|SpawnObstacleLong)
        (elif (Utilities|ClassIsChildOf (Variables|Default|GetObstacle) "/Game/Blueprints/Game/ObstacleGrandLong.ObstacleGrandLong_C")
          (CallFunction|SpawnObstacleLong))))))

(fn RalentirCharacter
  (params (DeltaTime :type Float%20%28single-precision%29))
  (bind _mycharacter (Variables|Default|GetMyCharacter))
  (bind _charactermovement (Variables|/Script/Engine.Character|GetCharacterMovement _mycharacter))
  (if (Variables|Default|GetRalentit)
    (if (Variables|Default|GetPremiereBoucleRalentit)
      (CallFunction|SlowCharacter)
      (Variables|Default|SetPremiereBoucleRalentit false)
      (else
        (Variables|Default|SetTimerSlow (+ (Variables|Default|GetTimerSlow) DeltaTime))
        (if (>= (Variables|Default|GetTimerSlow) 1e+01)
          (Variables|Default|SetRalentit false)
          (Variables|Default|SetTempMaxSpeed (+ (Variables|Default|GetTempMaxSpeed) 5e+02))
          (Variables|/Script/Engine.CharacterMovementComponent|SetMaxWalkSpeed (Variables|/Script/Engine.Character|GetCharacterMovement (Variables|Default|GetMyCharacter)) 0.0))))
    (elif (Variables|Default|GetPremiereBouclePasRalentit)
      (if (< (Variables|/Script/Engine.CharacterMovementComponent|GetMaxWalkSpeed _charactermovement) 1e+03)
        (Variables|/Script/Engine.CharacterMovementComponent|SetMaxWalkSpeed _charactermovement 1e+03)
        (Variables|Default|SetTempMaxSpeed 1e+03)
        (Variables|Default|SetTimerSlow 0.0)
        (Variables|Default|SetPremiereBouclePasRalentit false)))))

(fn DecelererCharacter
  (params (DeltaTime :type Float%20%28single-precision%29))
  (if (Variables|Default|GetVitesseUtilise)
    (Variables|Default|SetRalentit false)
    (if (<= (Variables|Default|GetTimerVitesse) 5.0)
      (Variables|Default|SetTimerVitesse (+ (Variables|Default|GetTimerVitesse) DeltaTime))
      (else
        (Variables|Default|SetVitesseUtilise false)
        (Variables|Default|SetTimerVitesse 0.0)
        (Variables|/Script/Engine.CharacterMovementComponent|SetMaxWalkSpeed (Variables|/Script/Engine.Character|GetCharacterMovement (Variables|Default|GetMyCharacter)) 1e+03)
        (Variables|Default|SetDeceleration true)))))

(fn InterrompreCombo
  (if (Variables|Default|GetContaminationDisponible)
    (Variables|/Game/Blueprints/ZombieHud.ZombieHud_C|SetFailed (Variables|Default|GetHUD) true)
    (Variables|Default|SetContaminationDisponible false)
    (Variables|/Game/Blueprints/ZombieHud.ZombieHud_C|SetDejaAfficherContam (Variables|Default|GetHUD) false)))

(fn DestructionObstacles
  (params (DeltaTime :type Float%20%28single-precision%29))
  (if (Variables|Default|GetDestructionActive)
    (if (<= (Variables|Default|GetTimerDestruction) 5.0)
      (Variables|Default|SetTimerDestruction (+ (Variables|Default|GetTimerDestruction) DeltaTime))
      (else
        (Variables|Default|SetDestructionActive false)
        (Variables|Default|SetTimerDestruction 0.0)
        (Variables|/Game/Blueprints/ZombieHud.ZombieHud_C|SetDejaAfficherColere (Variables|Default|GetHUD) false)))))

(fn AccelererCharacter
  (if (Variables|Default|GetVitesseDisponible)
    (Variables|/Script/Engine.CharacterMovementComponent|SetMaxWalkSpeed (Variables|/Script/Engine.Character|GetCharacterMovement (Variables|Default|GetMyCharacter)) 2e+03)
    (Variables|Default|SetVitesseUtilise true)
    (Variables|Default|SetVitesseDisponible false)
    (Variables|/Game/Blueprints/ZombieHud.ZombieHud_C|SetDejaAfficherVitesse (Variables|Default|GetHUD) false)
    (Variables|Default|SetDeceleration false)))