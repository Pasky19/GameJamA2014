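; FinLevel is an end-of-level trigger that detects when the player character reaches it.
; On overlap, BoxCollider checks the other component against the player 0 character's root component and sets the FinLevel flag.
; It then casts the player's HUD to ZombieHud, keeps a reference, and copies its TempsDeJeu play time into its own Time variable.
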(event OnComponentBeginOverlap(BoxCollider)
  (params (OtherActor :type Actor%20Object%20Reference) (OtherComp :type Primitive%20Component%20Object%20Reference) (OtherBodyIndex :type Integer) (bFromSweep :type Boolean) (SweepResult :type Hit%20Result%20Structure%20%28by%20ref%29))
  (if (== OtherComp (VehicleSound|GetRootComponent (Game|GetPlayerCharacter 0)))
    (Variables|Default|SetFinLevel true)
    (bind _aszombiehud_c (Utilities|Casting|CastToZombieHud (HUD|GetHUD (Game|GetPlayerController 0))))
    (Variables|Default|SetHUD _aszombiehud_c)
    (Variables|Default|SetTime (Variables|/Game/Blueprints/ZombieHud.ZombieHud_C|GetTempsDeJeu (Variables|Default|GetHUD)))))

(fn ConstructionScript)