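; MenuHud is a main menu HUD drawn on the canvas, with French "Comment Jouer" (how to play) and "Jouer" (play) options.
; DrawHUD paints a tiled fire texture, then draws each label relative to screen center with a named hit box at the same position.
; HitBoxClick branches on the box name: Jouer opens Example_Map, while Info only prints a debug string.
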(event EventDrawHUD
  (params (SizeX :type Integer) (SizeY :type Integer))
  (bind _returnvalue (/ SizeX 2))
  (bind _returnvalue_2 (Math|Conversions|ToFloat(Integer) _returnvalue))
  (bind _returnvalue_3 (- _returnvalue_2 5e+01))
  (bind _returnvalue_4 (- _returnvalue_2 1.5e+02))
  (Class|HUD|DrawTextureSimple "/Game/Textures/T_Fire_Tiled_D.T_Fire_Tiled_D" 0.0 0.0 3.0 false)
  (HUD|DrawText "Comment Jouer" "(R=0.244920,G=0.980000,B=0.000000,A=1.000000)" _returnvalue_4 2.5e+02 0 3.0 false)
  (Class|HUD|AddHitBox (Math|Vector2D|MakeVector2D _returnvalue_4 2.5e+02) "(X=300.000000,Y=100.000000)" "Info" false)
  (HUD|DrawText "Jouer" "(R=0.204968,G=0.985000,B=0.059257,A=1.000000)" _returnvalue_3 3.5e+02 0 3.0 false)
  (Class|HUD|AddHitBox (Math|Vector2D|MakeVector2D _returnvalue_3 3.5e+02) "(X=300.000000,Y=100.000000)" "Jouer" false))

(event EventHitBoxClick
  (params (BoxName :type Name :default "None"))
  (if (Utilities|Name|Equal(Name) BoxName "Info")
    (Development|PrintString "Info")
    (elif (Utilities|Name|Equal(Name) BoxName "Jouer")
      (Game|OpenLevel(byName) "Example_Map"))))

(fn ConstructionScript)