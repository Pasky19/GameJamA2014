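; HUD for the main menu, drawing Jouer (play), Intro and Quitter (quit) buttons with matching hit boxes.
; Intro steps through three story screens and an instruction screen, moving the owning pawn for the second and third.
; Jouer shows only the instructions; both paths then open Example_Map.
; A full-screen hit box increments State on each click to advance the screens.
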(event Custom|MoveHistoire
  (params (state :type Integer))
  (bind _camera (Variables|Default|GetCamera))
  (bind _returnvalue (VehicleSound|GetRootComponent _camera))
  (if (== state 2)
    (Components|MoveComponentTo _returnvalue "-250.000000,3000.000000,90.000000" "0, 0, 0" false false 0.1)
    (else
      (Components|MoveComponentTo _returnvalue "1800.000000,6100.000000,110.000000" "0, 0, 0" false false 0.2))))

(event EventHitBoxRelease
  (params (BoxName :type Name :default "None"))
  (if (Utilities|Name|Equal(Name) BoxName "Jouer")
    (Variables|Default|SetStart false)
    (Variables|Default|SetJouer true)
    (elif (Utilities|Name|Equal(Name) BoxName "Intro")
      (Variables|Default|SetStart false)
      (Variables|Default|SetIntro true)
      (elif (Utilities|Name|Equal(Name) BoxName "Quitter")
        (Game|QuitGame (Game|Player|GetOwningPlayerController))
        (elif (Utilities|Name|Equal(Name) BoxName "State")
          (Variables|Default|SetState (+ (Variables|Default|GetState) 1)))))))

(event EventBeginPlay
  (Variables|Default|SetCamera (Class|HUD|GetOwningPawn)))

(event EventDrawHUD
  (params (SizeX :type Integer) (SizeY :type Integer))
  (if (Variables|Default|GetStart)
    (Class|HUD|DrawTextureSimple "/Game/Textures/Jouer.Jouer" 1.9e+02 2e+02 1.0 false)
    (Class|HUD|AddHitBox (Math|Vector2D|MakeVector2D 1.9e+02 2e+02) "(X=130.000000,Y=100.000000)" "Jouer" false)
    (Class|HUD|DrawTextureSimple "/Game/Textures/Intro.Intro" 1.9e+02 3e+02 1.0 false)
    (Class|HUD|AddHitBox "(X=190.000000,Y=300.000000)" "(X=130.000000,Y=100.000000)" "Intro" false)
    (Class|HUD|DrawTextureSimple "/Game/Textures/Quitter.Quitter" 0.0 2.1e+02 1.0 true)
    (Class|HUD|AddHitBox "(X=185.000000,Y=430.000000)" "(X=140.000000,Y=100.000000)" "Quitter" false)
    (elif (Variables|Default|GetIntro)
      (if (== (Variables|Default|GetState) 1)
        (Class|HUD|DrawTextureSimple "/Game/Textures/Histoire1.Histoire1" 0.0 0.0 1.0 false)
        (Class|HUD|AddHitBox :Size (Math|Vector2D|MakeVector2D (Math|Conversions|ToFloat(Integer) SizeX) (Math|Conversions|ToFloat(Integer) SizeY)) :Name "State" :!label _label)
        (elif (== (Variables|Default|GetState) 2)
          (Class|HUD|DrawTextureSimple "/Game/Textures/Histoire2.Histoire2" 0.0 0.0 1.0 false)
          (CallFunction|MoveHistoire (Variables|Default|GetState) :!label _label_2)
          (goto _label)
          (elif (== (Variables|Default|GetState) 3)
            (Class|HUD|DrawTextureSimple "/Game/Textures/Histoire3.Histoire3" 0.0 0.0 1.0 false)
            (goto _label_2)
            (elif (== (Variables|Default|GetState) 4)
              (Class|HUD|DrawTextureSimple "/Game/Textures/Instruction.Instruction" 3e+02 0.0 0.4 false)
              (goto _label)
              (elif (== (Variables|Default|GetState) 5)
                (Variables|Default|SetState 0)
                (Variables|Default|SetIntro false)
                (Game|OpenLevel(byName) "Example_Map"))))))
      (elif (== (Variables|Default|GetState) 1)
        (Class|HUD|DrawTextureSimple "/Game/Textures/Instruction.Instruction" 3e+02 0.0 0.4 false)
        (goto _label)
        (else
          (Game|OpenLevel(byName) "Example_Map"))))))

(fn ConstructionScript)