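; Zombie game HUD that runs an arrow-key rhythm minigame, shows elapsed time and opens the LeaderBoard level after 70 seconds.
; Tick launches random combos; each arrow flashes while a Go window is open, with Failed preset until cleared externally.
; Successful combos randomly trigger obstacles (faster next combo), slowdown or brain moves (pace reset) through ZomieGame.
; Failures reset pace and unlock a random ability, whose image shows briefly once.
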(event Custom|SetNextCombo
  (params (NewTimerNextKey :type Float%20%28single-precision%29))
  ;[1 1 1] Calculer la prochaines suite
  (Variables|Default|SetComboCount (+ (Math|Random|RandomInteger 4) 2))
  (Variables|Default|SetDelayNextkey NewTimerNextKey)
  (Utilities|FlowControl|Delay (Variables|Default|GetTimerNextCombo))
  (Variables|Default|SetCombo true))

(event Custom|InitializeFleche
  ;[1 1 1] Réinitialisaiton des flèches de départ
  (Variables|Default|SetTexTureLeftKey "/Game/Textures/FlécheGaucheInit.FlécheGaucheInit")
  (Variables|Default|SetTextureRightKey "/Game/Textures/FlécheDroiteInit.FlécheDroiteInit")
  (Variables|Default|SetTextureUpKey "/Game/Textures/FlécheUpInit.FlécheUpInit")
  (Variables|Default|SetTextureDownKey "/Game/Textures/FlécheDownInit.FlécheDownInit"))

(event Custom|SetCombo%20Arrows
  (params (Count :type Integer) (NewArrow :type Float%20%28single-precision%29))
  (bind _zombiegame (Variables|Default|GetZombieGame))
  (bind _zombiegame_2 (Variables|Default|GetZombieGame))
  ;[1 1 1] Initialise la suite de flèche
  (Variables|Default|SetCombo false)
  (Variables|Default|SetComboCount Count)
  (CallFunction|InitializeFleche :!label _label)
  (Variables|Default|SetFailed true)
  (Variables|Default|SetRandomKey (Math|Random|RandomInteger 4))
  (if (== (Variables|Default|GetRandomKey) 0)
    (Variables|Default|SetTexTureLeftKey "/Game/Textures/FlécheGaucheFlash.FlécheGaucheFlash")
    (Variables|Default|SetKeyName "Left")
    ;[1 1 1] Décrémente le count, envoiele go pour detecter les touches, si failed arrete la suite, sinon continue
    (Variables|Default|SetComboCount (- (Variables|Default|GetComboCount) 1) :!label _label_2)
    (Variables|Default|SetGo? true)
    (Utilities|FlowControl|Delay NewArrow)
    (Variables|Default|SetGo? false)
    (if (Variables|Default|GetFailed)
      ;[1 1 1] Si la suite c'Est terminé abuptement ou spawndobjet special
      (CallFunction|InitializeFleche)
      (Variables|Default|SetSuiteCombo 0)
      (bind _abilityname (CallFunction|ZombieAbility))
      (Variables|Default|SetDeccelerate true)
      (CallFunction|SetNextCombo 1.0)
      (if (Utilities|Name|Equal(Name) _abilityname "Vitesse")
        (Variables|/Game/Blueprints/ZomieGame.ZomieGame_C|SetVitesseDisponible _zombiegame_2 true)
        (elif (Utilities|Name|Equal(Name) _abilityname "Contamination")
          (Variables|/Game/Blueprints/ZomieGame.ZomieGame_C|SetContaminationDisponible _zombiegame_2 true)
          (elif (Utilities|Name|Equal(Name) _abilityname "Colere")
            (Variables|/Game/Blueprints/ZomieGame.ZomieGame_C|SetDestructionDisponible _zombiegame_2 true))))
      (elif (== (Variables|Default|GetComboCount) 0)
        (Class|GameplayStatics|PlaySoundAttached "/Game/Audio/YEAH.YEAH" (VehicleSound|GetRootComponent))
        ;[1 1 1] Si combo réussi, caller la fonction de determination d'habilite, en suite recalculer la prochaine suite
        (CallFunction|InitializeFleche)
        (Variables|Default|SetSuiteCombo (+ (Variables|Default|GetSuiteCombo) 1))
        (bind (_specialhabilitiesout _spawningobjectout) (CallFunction|AbilityRythm (Variables|Default|GetSuiteCombo)))
        (if (Utilities|Name|Equal(Name) _spawningobjectout "Obstacle")
          (Default|SpawnObstacle _zombiegame)
          (if _specialhabilitiesout :!label _label_3
            (CallFunction|InitializeFleche)
            (Variables|Default|SetSuiteCombo 0)
            (Variables|Default|SetDeccelerate true)
            (CallFunction|SetNextCombo 1.0)
            (else
              (Variables|Default|SetAccelerate true)
              (CallFunction|SetNextCombo (- NewArrow 0.3))))
          (elif (Utilities|Name|Equal(Name) _spawningobjectout "Brain")
            (Default|MovetoCerveau _zombiegame)
            (goto _label_3)
            (elif (Utilities|Name|Equal(Name) _spawningobjectout "Injured")
              (Variables|/Game/Blueprints/ZomieGame.ZomieGame_C|SetRalentit _zombiegame true)
              (Variables|/Game/Blueprints/ZomieGame.ZomieGame_C|SetPremiereBoucleRalentit _zombiegame true)
              (Variables|/Game/Blueprints/ZomieGame.ZomieGame_C|SetPremiereBouclePasRalentit _zombiegame true)
              (goto _label_3))))
        (else
          (goto _label))))
    (elif (== (Variables|Default|GetRandomKey) 1)
      (Variables|Default|SetTextureUpKey "/Game/Textures/FlécheUpFlash.FlécheUpFlash")
      (Variables|Default|SetKeyName "Up")
      (goto _label_2)
      (elif (== (Variables|Default|GetRandomKey) 2)
        (Variables|Default|SetTextureDownKey "/Game/Textures/FlécheDownFlash.FlécheDownFlash")
        (Variables|Default|SetKeyName "Down")
        (goto _label_2)
        (elif (== (Variables|Default|GetRandomKey) 3)
          (Variables|Default|SetTextureRightKey "/Game/Textures/FlécheDroiteFlash.FlécheDroiteFlash")
          (Variables|Default|SetKeyName "Right")
          (goto _label_2))))))

(event EventDrawHUD
  (params (SizeX :type Integer) (SizeY :type Integer))
  ;[1 1 1] Position des flèches de départ
  (if (>= (Variables|Default|GetTempsDeJeu) 7e+01)
    (Game|OpenLevel(byName) "LeaderBoard")
    (else
      (Variables|Default|SetScreenSizeX SizeX)
      (Variables|Default|SetScreenSizeY SizeY)
      (Class|HUD|DrawTextureSimple (Variables|Default|GetTexTureLeftKey) 25.0 25.0 0.025 false)
      (Class|HUD|DrawTextureSimple (Variables|Default|GetTextureUpKey) 1e+02 25.0 0.025 false)
      (Class|HUD|DrawTextureSimple (Variables|Default|GetTextureDownKey) 175.0 25.0 0.025 false)
      (Class|HUD|DrawTextureSimple (Variables|Default|GetTextureRightKey) 2.5e+02 25.0 0.025 false)
      (HUD|DrawText (Utilities|String|ToString(Float) (Variables|Default|GetTempsDeJeu)) "(R=0.555000,G=0.000000,B=0.000000,A=1.000000)" (- (Math|Conversions|ToFloat(Integer) (Variables|Default|GetScreenSizeX)) 1e+02) 25.0 0 1.0 false)
      (if (Variables|/Game/Blueprints/ZomieGame.ZomieGame_C|GetVitesseDisponible (Variables|Default|GetZombieGame))
        (if (not (Variables|Default|GetDejaAfficherVitesse))
          (if (Variables|Default|GetAffichageCommencerVitesse)
            _
            (else
              (Variables|Default|SetAffichageCommencerVitesse true)
              (Variables|Default|SetTimerAfficherVitesse 0.0)))
          (if (Variables|Default|GetAfficherVitesse)
            (Class|HUD|DrawTextureSimple "/Game/Textures/Vitesse.Vitesse" 0.0 0.0 1.0 false))
          (if (Variables|/Game/Blueprints/ZomieGame.ZomieGame_C|GetDestructionDisponible (Variables|Default|GetZombieGame)) :!label _label
            (if (not (Variables|Default|GetDejaAfficherColere))
              (if (Variables|Default|GetAffichageCommencerColere)
                _
                (else
                  (Variables|Default|SetAffichageCommencerColere true)
                  (Variables|Default|SetTimerAfficherColere 0.0)))
              (if (Variables|Default|GetAfficherColere)
                (Class|HUD|DrawTextureSimple "/Game/Textures/Colère.Colère" 0.0 0.0 1.0 false))
              (if (Variables|/Game/Blueprints/ZomieGame.ZomieGame_C|GetContaminationDisponible (Variables|Default|GetZombieGame)) :!label _label_2
                (if (not (Variables|Default|GetDejaAfficherContam))
                  (if (Variables|Default|GetAffichageCommencerContam)
                    _
                    (else
                      (Variables|Default|SetAffichageCommencerContam true)
                      (Variables|Default|SetTimerAfficherContam 0.0)))
                  (if (Variables|Default|GetAfficherContam)
                    (Class|HUD|DrawTextureSimple "/Game/Textures/Contamination.Contamination" 0.0 0.0 1.0 false)))))
            (else
              (goto _label_2))))
        (else
          (goto _label))))))

(event EventBeginPlay
  ;[1 1 1] Initialisation du jeu ryhtmique
  (CallFunction|InitializeFleche)
  (CallFunction|SetNextCombo 1.0)
  (bind _aszomiegame_c (Utilities|Casting|CastToZomieGame (Game|GetPlayerController 0)))
  (Variables|Default|SetZombieGame _aszomiegame_c))

(event EventTick
  (params (DeltaSeconds :type Float%20%28single-precision%29))
  ;[1 1 1] Si le temp d'un nouveau combo est arriver l'exécuter
  (Variables|Default|SetTempsDeJeu (+ DeltaSeconds (Variables|Default|GetTempsDeJeu)))
  (if (Variables|Default|GetAffichageCommencerVitesse)
    (Variables|Default|SetAfficherVitesse true)
    (Variables|Default|SetTimerAfficherVitesse (+ (Variables|Default|GetTimerAfficherVitesse) DeltaSeconds) :!label _label)
    (if (>= (Variables|Default|GetTimerAfficherVitesse) 2.0)
      (Variables|Default|SetAfficherVitesse false)
      (Variables|Default|SetAffichageCommencerVitesse false)
      (Variables|Default|SetDejaAfficherVitesse true))
    (elif (Variables|Default|GetAfficherVitesse)
      (goto _label)
      (else
        _)))
  (if (Variables|Default|GetAffichageCommencerColere)
    (Variables|Default|SetAfficherColere true)
    (Variables|Default|SetTimerAfficherColere (+ (Variables|Default|GetTimerAfficherColere) DeltaSeconds) :!label _label_2)
    (if (>= (Variables|Default|GetTimerAfficherColere) 2.0)
      (Variables|Default|SetAfficherColere false)
      (Variables|Default|SetAffichageCommencerColere false)
      (Variables|Default|SetDejaAfficherColere true))
    (elif (Variables|Default|GetAfficherColere)
      (goto _label_2)
      (else
        _)))
  (if (Variables|Default|GetAffichageCommencerContam)
    (Variables|Default|SetAfficherContam true)
    (Variables|Default|SetTimerAfficherContam (+ (Variables|Default|GetTimerAfficherContam) DeltaSeconds) :!label _label_3)
    (if (>= (Variables|Default|GetTimerAfficherContam) 2.0)
      (Variables|Default|SetAfficherContam false)
      (Variables|Default|SetAffichageCommencerContam false)
      (Variables|Default|SetDejaAfficherContam true))
    (elif (Variables|Default|GetAfficherContam)
      (goto _label_3)
      (else
        _)))
  (if (Variables|Default|GetCombo)
    (CallFunction|SetComboArrows (Variables|Default|GetComboCount) (Variables|Default|GetDelayNextkey))))

(fn ConstructionScript)

(fn AbilityRythm
  (params (Combos :type Integer))
  (bind _returnvalue (Math|Random|RandomInteger 10))
  (if (<= _returnvalue 5)
    (LocalVariables|SetSpawningObject "Obstacle")
    (LocalVariables|SetSpeciallabilities false)
    (else
      (if (<= _returnvalue 8)
        (LocalVariables|SetSpawningObject "Injured")
        (else
          (LocalVariables|SetSpawningObject "Brain")))
      (LocalVariables|SetSpeciallabilities true)))
  (return (LocalVariables|GetSpeciallabilities) (LocalVariables|GetSpawningObject)))

(fn Musique)

(fn ZombieAbility
  (LocalVariables|SetRandomAbility (Math|Random|RandomInteger 3))
  (if (== (LocalVariables|GetRandomAbility) 0)
    (LocalVariables|SetNameAbility "Colere")
    (return (LocalVariables|GetNameAbility))
    (elif (== (LocalVariables|GetRandomAbility) 1)
      (LocalVariables|SetNameAbility "Vitesse")
      (return (LocalVariables|GetNameAbility))
      (elif (== (LocalVariables|GetRandomAbility) 2)
        (LocalVariables|SetNameAbility "Contamination")
        (return (LocalVariables|GetNameAbility))))))