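; Leaderboard HUD that shows the saved best time under a French "Meilleur Temps" label, with a quit button.
; DrawHUD reloads the "ZombieGame" save slot on every draw, casts it to ZombieSaveGame and draws BestTime as green text.
; It then draws the Quitter texture and adds a hit box, offset lower than the texture's origin, whose click quits the game.
; If the cast fails, only the label is drawn.
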(event EventDrawHUD
  (params (SizeX :type Integer) (SizeY :type Integer))
  (bind _returnvalue (/ SizeX 2))
  (bind _returnvalue_2 (Math|Conversions|ToFloat(Integer) _returnvalue))
  (HUD|DrawText "Meilleur Temps:" "(R=0.244920,G=0.980000,B=0.000000,A=1.000000)" (- _returnvalue_2 1.5e+02) 1.5e+02 0 3.0 false)
  (bind _returnvalue_3 (SaveGame|LoadGamefromSlot "ZombieGame"))
  (Variables|Default|SetZombieSaveGame _returnvalue_3)
  (bind _aszombiesavegame_c (Utilities|Casting|CastToZombieSaveGame (Variables|Default|GetZombieSaveGame)))
  (HUD|DrawText (Utilities|String|ToString(Float) (Variables|/Game/Blueprints/Game/ZombieSaveGame.ZombieSaveGame_C|GetBestTime _aszombiesavegame_c)) "(R=0.160842,G=0.990000,B=0.044550,A=1.000000)" (- _returnvalue_2 1e+02) 3e+02 0 3.0 false)
  (Class|HUD|DrawTextureSimple "/Game/Textures/Quitter.Quitter" 7e+02 3.5e+02 1.0 false)
  (Class|HUD|AddHitBox "(X=700.000000,Y=500.000000)" "(X=500.000000,Y=500.000000)" "Quitter" false))

(event EventHitBoxClick
  (params (BoxName :type Name :default "None"))
  (if (Utilities|Name|Equal(Name) BoxName "Quitter")
    (Game|QuitGame)))

(fn ConstructionScript)